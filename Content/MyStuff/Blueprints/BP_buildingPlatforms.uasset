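; Puzzle platform that grows along Z while a BP_FiringCube with a material matching its CheckingScaleCube sits in the box collider.
; Overlap plays right-or-wrong audio and, on a match, starts LoopMove, a self-calling next-tick loop that steps PointB's clamped scale; any cube leaving shrinks it.
; The construction script previews full MaxZScale height, and BeginPlay collapses it.
; Timeline-based scaling events exist but are not called here.
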(event `scalingPlatform`
  (bind _pointb (`self.pointB`))
  (bind (_returnvalue_x _returnvalue_y _returnvalue_z) (`KismetMathLibrary.BreakVector` (`SceneComponent.K2_GetComponentScale` _pointb)))
  (bind (_returnvalue_x_2 _returnvalue_y_2 _returnvalue_z_2) (`KismetMathLibrary.BreakVector` (`SceneComponent.K2_GetComponentScale` (`self.pointB`))))
  ; Scaling the platforms
  (`Timeline|scaleTimeline` :`NewTime` (`KismetMathLibrary.SafeDivide` (`self.maxZScale`) 2.0) :!label _label
    (:`Update`
      (`SceneComponent.SetWorldScale3D` _pointb (`KismetMathLibrary.MakeVector` _returnvalue_x _returnvalue_y (+ _returnvalue_z 0.1)))
      (if (not (<= (`self.maxZScale`) _returnvalue_z_2))
        (`self.scalingPlatform`)))))

(event `reversingPlatforms`
  ; Scaling the platforms
  (goto _label :!via `Reverse`))

(event `LoopMove`
  (params (MoveValue :type "Float (double-precision)"))
  (bind _pointb (`self.pointB`))
  (bind (_returnvalue_x _returnvalue_y _returnvalue_z) (`KismetMathLibrary.BreakVector` (`SceneComponent.K2_GetComponentScale` _pointb)))
  (bind (_returnvalue_x_2 _returnvalue_y_2 _returnvalue_z_2) (`KismetMathLibrary.BreakVector` (`SceneComponent.K2_GetComponentScale` (`self.pointB`))))
  ; Scaling/Unscaling the platform
  (`KismetSystemLibrary.DelayUntilNextTick`)
  (`SceneComponent.SetWorldScale3D` _pointb (`KismetMathLibrary.MakeVector` _returnvalue_x _returnvalue_y (`KismetMathLibrary.FClamp` (+ _returnvalue_z MoveValue) 0.5 (`self.maxZScale`))))
  (if (not (== _returnvalue_z_2 (select `bool` (> MoveValue 0.0) :`false` 0.5 :`true` (`self.maxZScale`))))
    (`self.LoopMove` MoveValue)))

(event `self.ReceiveBeginPlay`
  (bind _pointb (`self.pointB`))
  (bind (_returnvalue_x _returnvalue_y) (`KismetMathLibrary.BreakVector` (`SceneComponent.K2_GetComponentScale` _pointb)))
  ; setting the scaling Back to normal
  (`SceneComponent.SetWorldScale3D` _pointb (`KismetMathLibrary.MakeVector` _returnvalue_x _returnvalue_y 0.5)))

(event `self.BoxCollider.OnComponentBeginOverlap`
  (params (OverlappedComponent :type "PrimitiveComponent Object Reference") (OtherActor :type "Actor Object Reference") (OtherComp :type "PrimitiveComponent Object Reference") (OtherBodyIndex :type Integer) (bFromSweep :type Boolean) (SweepResult :type "HitResult Structure (by ref)"))
  (bind _audio (`self.Audio`))
  ; Checking collition
  (bind _asbp_firing_cube (cast `/Game/MyStuff/Blueprints/BP_FiringCube` OtherActor))
  (if (== (`/Game/MyStuff/Blueprints/BP_FiringCube.Collition` _asbp_firing_cube) OtherComp)
    (`KismetSystemLibrary.PrintString` "GoingUp")
    (`KismetSystemLibrary.PrintString` "Cube is here")
    (bind _returnvalue (== (`PrimitiveComponent.GetMaterial` (`self.checkingScaleCube`) 0) (`PrimitiveComponent.GetMaterial` (`/Game/MyStuff/Blueprints/BP_FiringCube.Cube` _asbp_firing_cube) 0)))
    (if _returnvalue
      (`AudioParameterControllerInterface.SetBoolParameter` _audio "isCorrect" _returnvalue)
      (`AudioComponent.Play` _audio 0.0)
      (`self.LoopMove` 0.1)
      (else
        (`AudioParameterControllerInterface.SetBoolParameter` _audio "isCorrect" _returnvalue)
        (`AudioComponent.Play` _audio 0.0)))))

(event `self.BoxCollider.OnComponentEndOverlap`
  (params (OverlappedComponent :type "PrimitiveComponent Object Reference") (OtherActor :type "Actor Object Reference") (OtherComp :type "PrimitiveComponent Object Reference") (OtherBodyIndex :type Integer))
  ; Checking Collition leaves
  (bind _asbp_firing_cube (cast `/Game/MyStuff/Blueprints/BP_FiringCube` OtherActor))
  (if (== (`/Game/MyStuff/Blueprints/BP_FiringCube.Collition` _asbp_firing_cube) OtherComp)
    (`KismetSystemLibrary.PrintString` "GoingUp")
    (`KismetSystemLibrary.PrintString` "Cube is here")
    (`self.LoopMove` -0.1)))

(fn `UserConstructionScript`
  (bind _pointb (`self.pointB`))
  (bind (_returnvalue_x _returnvalue_y) (`KismetMathLibrary.BreakVector` (`SceneComponent.K2_GetComponentScale` _pointb)))
  (`SceneComponent.SetWorldScale3D` _pointb (`KismetMathLibrary.MakeVector` _returnvalue_x _returnvalue_y (`self.maxZScale`))))