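; Collectible coin pickup that spins its cylinder mesh every tick and adds to the player's score when collected.
; When the third-person character's capsule overlaps the sphere, it hides the mesh, disables collision and prints debug messages.
; It increments Score in BP_GameInstance, records itself in CollectedCoins and saves the game.
; On BeginPlay it destroys itself if already in that collected list.
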(event `self.ReceiveBeginPlay`
  (bind _asbp_game_instance (cast `/Game/MyStuff/SaveSystem/BP_GameInstance` (`GameplayStatics.GetGameInstance`)))
  (if (not (== (`KismetArrayLibrary.Array_Find` (`/Game/MyStuff/SaveSystem/BP_GameInstance.CollectedCoins` _asbp_game_instance) self) -1))
    (`self.K2_DestroyActor`)))

(event `self.Sphere Collition.OnComponentBeginOverlap`
  (params (OverlappedComponent :type "PrimitiveComponent Object Reference") (OtherActor :type "Actor Object Reference") (OtherComp :type "PrimitiveComponent Object Reference") (OtherBodyIndex :type Integer) (bFromSweep :type Boolean) (SweepResult :type "HitResult Structure (by ref)"))
  ; Pivk up
  (bind _asbp_third_person_character (cast `/Game/ThirdPerson/Blueprints/BP_ThirdPersonCharacter` OtherActor))
  (if (== (`Character.CapsuleComponent` _asbp_third_person_character) OtherComp)
    (`self.ChangeState` true)
    (`KismetSystemLibrary.PrintString` "Hello" true true (struct :`G` 0.66 :`B` 1.0 :`A` 1.0) 3.0)
    (bind _asbp_game_instance (cast `/Game/MyStuff/SaveSystem/BP_GameInstance` (`GameplayStatics.GetGameInstance`)))
    (bind _result (`/Engine/EditorBlueprintResources/StandardMacros.IncrementFloat` (`/Game/MyStuff/SaveSystem/BP_GameInstance.Score` _asbp_game_instance))
      (:`  `
        (`KismetSystemLibrary.PrintString` (`KismetStringLibrary.Conv_DoubleToString` _result))
        (`KismetArrayLibrary.Array_AddUnique` (`/Game/MyStuff/SaveSystem/BP_GameInstance.CollectedCoins` _asbp_game_instance) self)
        (`/Game/MyStuff/SaveSystem/BP_GameInstance.SaveGame` _asbp_game_instance)))))

(event `self.ReceiveTick`
  (params (DeltaSeconds :type "Float (single-precision)"))
  (`SceneComponent.K2_AddRelativeRotation` (`self.Cylinder`) (`KismetMathLibrary.MakeRotator` 0.0 0.0 (* DeltaSeconds 60.0 2.0)) false false))

(fn `ChangeState`
  (params (Collected :type Boolean))
  (`SceneComponent.SetVisibility` (`self.Cylinder`) (not Collected) false)
  (`PrimitiveComponent.SetCollisionEnabled` (`self.Sphere Collition`) (select `bool` (`local.Collected`) :`false` "QueryOnly" :`true` "NoCollision" :!type "ECollisionEnabled Enum")))

(fn `UserConstructionScript`)