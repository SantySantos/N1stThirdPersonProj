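; BP_FiringCube is a cube that can be adjusted while it is the player's SpawnedObject, then fired like a bullet.
; StartPhysics enables physics simulation and launches it at high speed along the controller's aim.
; Holding L/J rolls it, I/K pitches it, and M nudges it along the character's forward vector.
; Both adjustments repeat through self-calling events with retriggerable delays, checking ownership each step.
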(event `self.ReceiveBeginPlay`
  ; Enabling Physics in the object
  (`self.EnableInput` (`GameplayStatics.GetPlayerController` 0)))

(event `StartPhysics`
  (bind _cube (`self.Cube`))
  ; Firing cube as a bullet
  (`PrimitiveComponent.SetSimulatePhysics` _cube true)
  (`PrimitiveComponent.SetPhysicsLinearVelocity` _cube (* (`KismetMathLibrary.Conv_RotatorToVector` (`Controller.GetControlRotation` (`GameplayStatics.GetPlayerController` 0))) 10000.0) false "None"))

(event `Key|L`
  (params (Key :type "Key Structure"))
  ; Rotating the spawnedObject
  (:`Pressed`
    (set `self.isPressed` true)
    (set `self.rotationValue` 10.0)
    (`self.RotateLoop` true))
  (:`Released`
    (set `self.isPressed` false)))

(event `RotateLoop`
  (params (X :type Boolean) (Y :type Boolean) (Z :type Boolean))
  (bind _rotationvalue (`self.rotationValue`))
  (bind _cube (`self.Cube`))
  ; Rotating the spawnedObject
  (`KismetSystemLibrary.RetriggerableDelay` 0.2)
  (bind _asbp_third_person_character (cast `/Game/ThirdPerson/Blueprints/BP_ThirdPersonCharacter` (`GameplayStatics.GetPlayerCharacter` 0)))
  (if (and (`self.isPressed`) (== (`/Game/ThirdPerson/Blueprints/BP_ThirdPersonCharacter.SpawnedObject` _asbp_third_person_character) self))
    (`SceneComponent.K2_SetRelativeRotation` _cube (`KismetMathLibrary.ComposeRotators` (`SceneComponent.RelativeRotation` _cube) (`KismetMathLibrary.MakeRotator` (select `bool` X :`true` _rotationvalue :!type "Float (single-precision)") (select `bool` Y :`true` _rotationvalue :!type "Float (single-precision)") (select `bool` Z :`true` _rotationvalue :!type "Float (single-precision)"))) false false)
    (`self.RotateLoop` X Y Z)))

(event `Key|J`
  (params (Key :type "Key Structure"))
  ; Rotating the spawnedObject
  (:`Pressed`
    (set `self.isPressed` true)
    (set `self.rotationValue` -10.0)
    (`self.RotateLoop` true))
  (:`Released`
    (set `self.isPressed` false)))

(event `Key|I`
  (params (Key :type "Key Structure"))
  ; Rotating the spawnedObject
  (:`Pressed`
    (set `self.isPressed` true)
    (set `self.rotationValue` 10.0)
    (`self.RotateLoop` false true))
  (:`Released`
    (set `self.isPressed` false)))

(event `Key|K`
  (params (Key :type "Key Structure"))
  ; Rotating the spawnedObject
  (:`Pressed`
    (set `self.isPressed` true)
    (set `self.rotationValue` -10.0)
    (`self.RotateLoop` false true))
  (:`Released`
    (set `self.isPressed` false)))

(event `PositionLoop`
  ; position loop custom event
  (`KismetSystemLibrary.RetriggerableDelay` 0.1)
  (bind _asbp_third_person_character (cast `/Game/ThirdPerson/Blueprints/BP_ThirdPersonCharacter` (`GameplayStatics.GetPlayerCharacter` 0)))
  (if (and (`self.canMove`) (== (`/Game/ThirdPerson/Blueprints/BP_ThirdPersonCharacter.SpawnedObject` _asbp_third_person_character) self))
    (`self.K2_SetActorLocation` (+ (`self.K2_GetActorLocation`) (* (`KismetMathLibrary.Conv_RotatorToVector` (`self.K2_GetActorRotation` _asbp_third_person_character)) (`self.moveValue`))))
    (`self.PositionLoop`)))

(event `Key|M`
  (params (Key :type "Key Structure"))
  ; Moving the object(in progress)
  (:`Pressed`
    (set `self.canMove` true)
    (set `self.moveValue` 10.0)
    (`self.PositionLoop`))
  (:`Released`
    (set `self.canMove` false)))

(fn `UserConstructionScript`)