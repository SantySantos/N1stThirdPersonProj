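; BP_Platform is a moving platform that shuttles its Cube back and forth between the actor's location and the ScenePoint component.
; A timeline starts on BeginPlay with its play rate set to the inverse of Speed, and its Percentage track drives a world-space lerp of the Cube without sweep.
; Each time the timeline finishes, it pauses briefly, then switches direction, looping indefinitely.
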(event `self.ReceiveBeginPlay`
  (`TimelineComponent.SetPlayRate` (`self.moveTimeline`) (/ 1.0 (`self.speed`)))
  (`self.StartTimeline`))

(event `StartTimeline`
  (bind (_direction _percentage) (`Timeline|moveTimeline` :!label _label)
    (:`Update`
      (`SceneComponent.K2_SetWorldLocation` (`self.Cube`) (`KismetMathLibrary.VLerp` (`self.K2_GetActorLocation`) (`SceneComponent.K2_GetComponentLocation` (`self.ScenePoint`)) _percentage) false false))
    (:`Finished`
      (`KismetSystemLibrary.Delay` 1.0)
      (switch `ETimelineDirection` _direction
        (:`Forward`
          (`self.ReverseTimeline`))
        (:`Backward`
          (`self.StartTimeline`))))))

(event `ReverseTimeline`
  (goto _label :!via `Reverse`))

(fn `UserConstructionScript`)