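; Interactive toggle button that switches a list of linked actors on and off.
; Its box collision enables input while the third-person character's capsule overlaps it and disables it on exit.
; Each Interact plays a spark sound, prints debug text, and flip-flops the cube's material color between green and red.
; The same flip-flop sends Activate or Deactivate messages to every InteractActors entry implementing BPI_Interact.
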(event `self.BoxCollition.OnComponentBeginOverlap`
  (params (OverlappedComponent :type "PrimitiveComponent Object Reference") (OtherActor :type "Actor Object Reference") (OtherComp :type "PrimitiveComponent Object Reference") (OtherBodyIndex :type Integer) (bFromSweep :type Boolean) (SweepResult :type "HitResult Structure (by ref)"))
  (bind _asbp_third_person_character (cast `/Game/ThirdPerson/Blueprints/BP_ThirdPersonCharacter` OtherActor))
  (if (== (`Character.CapsuleComponent` _asbp_third_person_character) OtherComp)
    (`self.EnableInput` (`GameplayStatics.GetPlayerController` 0))))

(event `self.BoxCollition.OnComponentEndOverlap`
  (params (OverlappedComponent :type "PrimitiveComponent Object Reference") (OtherActor :type "Actor Object Reference") (OtherComp :type "PrimitiveComponent Object Reference") (OtherBodyIndex :type Integer))
  (bind _asbp_third_person_character (cast `/Game/ThirdPerson/Blueprints/BP_ThirdPersonCharacter` OtherActor))
  (if (== (`Character.CapsuleComponent` _asbp_third_person_character) OtherComp)
    (`self.DisableInput` (`GameplayStatics.GetPlayerController` 0))))

(event `/Game/MyStuff/Blueprints/BP_Interfaces/BPI_Interactable.Interact`
  (bind _interactactors (`self.interactActors`))
  (bind _cube (`self.Cube`))
  (`KismetSystemLibrary.PrintString` "Interact")
  (`GameplayStatics.PlaySound2D` "/Game/StarterContent/Audio/Fire_Sparks01.Fire_Sparks01" 1.0 1.0 0.0 null null)
  (`/Engine/EditorBlueprintResources/StandardMacros.FlipFlop`
    (:`A`
      (`MeshComponent.SetVectorParameterValueOnMaterials` _cube "Base Color" (`KismetMathLibrary.Conv_LinearColorToVector` (struct :`G` 1.0 :`B` 0.051112 :`A` 1.0)))
      (for _array_element _interactactors
        (if (`KismetSystemLibrary.DoesImplementInterface` _array_element "/Game/MyStuff/Blueprints/BP_Interfaces/BPI_Interact.BPI_Interact_C")
          (message `/Game/MyStuff/Blueprints/BP_Interfaces/BPI_Interact.Activate` _array_element))))
    (:`B`
      (`MeshComponent.SetVectorParameterValueOnMaterials` _cube "Base Color" (`KismetMathLibrary.Conv_LinearColorToVector` (struct :`R` 0.65625 :`B` 0.058631 :`A` 1.0)))
      (for _array_element_2 _interactactors
        (if (`KismetSystemLibrary.DoesImplementInterface` _array_element_2 "/Game/MyStuff/Blueprints/BP_Interfaces/BPI_Interact.BPI_Interact_C")
          (message `/Game/MyStuff/Blueprints/BP_Interfaces/BPI_Interact.Deactivate` _array_element_2))))))

(fn `UserConstructionScript`)